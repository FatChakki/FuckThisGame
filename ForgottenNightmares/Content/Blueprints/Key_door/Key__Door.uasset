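; Locked door actor that the player can swing open and closed once their first-person character has DoorKey1.
; A box overlap enables input and shows either an Open or Need Key widget based on the key, and end overlap disables input and removes both.
; The Interaction action plays or reverses a timeline that yaws DoorA up to 90 degrees.
; DoorTime blocks presses mid-swing, while DoorOpen, updated from the track value, picks the direction.
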(event OnComponentBeginOverlap(Box)
  (params (OverlappedComponent :type Primitive%20Component%20Object%20Reference) (OtherActor :type Actor%20Object%20Reference) (OtherComp :type Primitive%20Component%20Object%20Reference) (OtherBodyIndex :type Integer) (bFromSweep :type Boolean) (SweepResult :type Hit%20Result%20Structure%20%28by%20ref%29))
  (Input|EnableInput (Game|GetPlayerController 0))
  (bind _asbp_first_person_character (Utilities|Casting|CastToBP_FirstPersonCharacter (Game|GetPlayerCharacter 0)))
  (if (Variables|/Game/FirstPerson/Blueprints/BP_FirstPersonCharacter.BP_FirstPersonCharacter_C|GetDoorKey1 _asbp_first_person_character)
    (bind _returnvalue (UserInterface|CreateWidget "/Game/Blueprints/Key_door/Open.Open_C"))
    (UserInterface|Viewport|AddtoViewport _returnvalue 0)
    (else
      (bind _returnvalue_2 (UserInterface|CreateWidget "/Game/Blueprints/Key_door/Need__Key.Need__Key_C"))
      (UserInterface|Viewport|AddtoViewport _returnvalue_2 0))))

(event OnComponentEndOverlap(Box)
  (params (OverlappedComponent :type Primitive%20Component%20Object%20Reference) (OtherActor :type Actor%20Object%20Reference) (OtherComp :type Primitive%20Component%20Object%20Reference) (OtherBodyIndex :type Integer))
  (Input|DisableInput (Game|GetPlayerController 0))
  (Widget|RemovefromParent (stale OnComponentBeginOverlap(Box) _returnvalue))
  (Widget|RemovefromParent (stale OnComponentBeginOverlap(Box) _returnvalue_2)))

(event EventBeginPlay
  (bind _returnvalue (UserInterface|CreateWidget "/Game/Blueprints/Key_door/Need__Key.Need__Key_C"))
  (Variables|Default|SetNeed _returnvalue))

(event Input|ActionEvents|InputActionInteraction
  (params (Key :type Key%20Structure :default "None"))
  (:Pressed
    (bind _asbp_first_person_character (Utilities|Casting|CastToBP_FirstPersonCharacter (Game|GetPlayerCharacter 0)))
    (if (Variables|/Game/FirstPerson/Blueprints/BP_FirstPersonCharacter.BP_FirstPersonCharacter_C|GetDoorKey1 _asbp_first_person_character)
      (if (Variables|Default|GetDoorTime)
        (if (Variables|Default|GetDoorOpen)
          (Variables|Default|SetDoorTime false)
          (bind _newtrack_0 (Timeline|Timeline_Door Play)
            (:Update
              (Transformation|SetRelativeRotation (Variables|Default|GetDoor_a) (Math|Rotator|MakeRotator 0.0 0.0 (* _newtrack_0 9e+01)) false false)
              (Variables|Default|SetDoorOpen (not (> _newtrack_0 0.0))))
            (:Finished
              (Variables|Default|SetDoorTime true)))
          (else
            (Variables|Default|SetDoorTime false)
            (Timeline|Timeline_Door ReverseFromEnd)))))))

(fn ConstructionScript)