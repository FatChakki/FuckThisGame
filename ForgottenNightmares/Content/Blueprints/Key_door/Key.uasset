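; Key is a pickup actor that grants the first-person player the key for a door.
; On BeginPlay it creates a prompt widget, which its Box overlap adds to the viewport while also enabling input, and removes with input disabled on exit.
; Pressing Interaction sets DoorKey1 on BP_FirstPersonCharacter and destroys the key.
; The overlap events do not check which actor triggered them.
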(event OnComponentBeginOverlap(Box)
  (params (OverlappedComponent :type Primitive%20Component%20Object%20Reference) (OtherActor :type Actor%20Object%20Reference) (OtherComp :type Primitive%20Component%20Object%20Reference) (OtherBodyIndex :type Integer) (bFromSweep :type Boolean) (SweepResult :type Hit%20Result%20Structure%20%28by%20ref%29))
  (Input|EnableInput (Game|GetPlayerController 0))
  (UserInterface|Viewport|AddtoViewport (Variables|Default|GetKey) 0))

(event OnComponentEndOverlap(Box)
  (params (OverlappedComponent :type Primitive%20Component%20Object%20Reference) (OtherActor :type Actor%20Object%20Reference) (OtherComp :type Primitive%20Component%20Object%20Reference) (OtherBodyIndex :type Integer))
  (Input|DisableInput (Game|GetPlayerController 0))
  (Widget|RemovefromParent (Variables|Default|GetKey)))

(event EventBeginPlay
  (bind _returnvalue (UserInterface|CreateWidget "/Game/Blueprints/Key_door/Key__Text.Key__Text_C"))
  (Variables|Default|SetKey _returnvalue))

(event Input|ActionEvents|InputActionInteraction
  (params (Key :type Key%20Structure :default "None"))
  (:Pressed
    (bind _asbp_first_person_character (Utilities|Casting|CastToBP_FirstPersonCharacter (Game|GetPlayerCharacter 0)))
    (Variables|/Game/FirstPerson/Blueprints/BP_FirstPersonCharacter.BP_FirstPersonCharacter_C|SetDoorKey1 _asbp_first_person_character true)
    (Actor|DestroyActor)))

(fn ConstructionScript)